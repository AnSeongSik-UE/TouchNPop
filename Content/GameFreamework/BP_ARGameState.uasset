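; BP_ARGameState is the game state for an AR game and keeps the player's score.
; On BeginPlay it resets PlayerScore, binds to the AddScore dispatcher on BP_ARPlayerController, then broadcasts UpdateScore with the starting value for the UI.
; EventAddScore increments the score by one but does not itself broadcast UpdateScore.
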(event `self.ReceiveBeginPlay`
  ; 게임시작 시 PlayerScore를 0으로 초기화
  (set `self.PlayerScore` 0)
  ; AddScore Dispatcher를 Bind : (Call = BP_ARPlayerController)
  (bind _asbp_arplayer_controller (cast `/Game/GameFreamework/BP_ARPlayerController` (`GameplayStatics.GetPlayerController` 0)))
  (add `/Game/GameFreamework/BP_ARPlayerController.AddScore` _asbp_arplayer_controller (`|CreateDelegate` :!event `EventAddScore`))
  ; PlayerScore를 UI에 업데이트
  (`self.UpdateScore` (`self.PlayerScore`)))

(fn `EventAddScore`
  (set `self.PlayerScore` (+ (`self.PlayerScore`) 1)))

(fn `UserConstructionScript`)