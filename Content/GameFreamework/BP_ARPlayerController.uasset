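; Player controller for the AR game that lets the player tap placed BP_Placeable actors to score and remove them.
; On touch press it traces WorldDynamic objects under Touch1, calls the CallAddScore dispatcher (noted as bound in BP_ARGameState) and destroys the hit placeable.
; It then has the controlled BP_ARPawn decrement its spawn count.
; A separate TouchedActorIsPlaceable helper does a similar Visibility-channel trace but is not called in this graph.
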(event `InputTouch`
  (params (Location :type "Vector Structure") (FingerIndex :type "ETouchIndex Enum"))
  (:`Pressed`
    ;[1 1 1] 터치된 Actor가 BP_Placeable 인지 확인
    (bind _asbp_placeable (cast `/Game/Placeable/BP_Placeable` (`.HitActor` (`GameplayStatics.BreakHitResult` (`self.GetHitResultUnderFingerForObjects` "Touch1" (`|MakeArray` "ObjectTypeQuery2" :!type "EObjectTypeQuery Enum"))))))
    ;[1 1 1] 점수 추가 Event 호출
    ; -> BP_ARGameState에서 Bind
    (`self.AddScore`)
    (`self.K2_DestroyActor` _asbp_placeable)
    (bind _asbp_arpawn (cast `/Game/GameFreamework/BP_ARPawn` (`self.K2_GetPawn`)))
    (`/Game/GameFreamework/BP_ARPawn.SpawnCountSubstract` _asbp_arpawn)))

(fn `TouchedActorIsPlaceable`
  (returns (`AsBP Placeable` :type "/Game/Placeable/BP_Placeable Object Reference"))
  (bind _asbp_placeable (cast `/Game/Placeable/BP_Placeable` (`.HitActor` (`GameplayStatics.BreakHitResult` (`self.GetHitResultUnderFingerByChannel` "Touch1" "TraceTypeQuery1"))))
    (:`then`
      (return _asbp_placeable))
    (:`CastFailed`
      (`KismetSystemLibrary.PrintString` "BP_ARPlayerController : Failed Casting BP_Placeable!" true true (struct :`R` 1.0 :`A` 1.0) 10.0))))

(fn `UserConstructionScript`)