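; AR game state Blueprint that tracks the player's score and the current game state.
; On BeginPlay it resets the score and binds to the AR player controller's AddScore dispatcher, incrementing and printing the score, then broadcasting UpdateScore.
; ChangeGameState resets DT, stores the new state and broadcasts StateChange, while Tick overwrites DT with the frame delta.
; EventAddScore duplicates the increment and print without broadcasting.
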(event `self.ReceiveBeginPlay`
  ; 게임시작 시 PlayerScore를 0으로 초기화
  (set `self.PlayerScore` 0)
  ; AddScore Dispatcher를 Bind : (Call = BP_ARPlayerController)
  (bind _asbp_arplayer_controller (cast `/Game/GameFreamework/BP_ARPlayerController` (`GameplayStatics.GetPlayerController` 0)))
  (add `/Game/GameFreamework/BP_ARPlayerController.AddScore` _asbp_arplayer_controller (delegate `AddScore`)))

(event `AddScore`
  ; AddScore Dispatcher를 Bind : (Call = BP_ARPlayerController)
  (bind _output_get (set `self.PlayerScore` (+ (`self.PlayerScore`) 1)))
  (`KismetSystemLibrary.PrintString` (`KismetStringLibrary.Conv_IntToString` _output_get) true true (struct :`R` 1.0 :`G` 0.012133 :`B` 0.024673 :`A` 1.0) 5.0)
  ; PlayerScore를 UI에 업데이트
  (`self.UpdateScore` _output_get))

(event `self.ReceiveTick`
  (params (DeltaSeconds :type "Float (single-precision)"))
  (set `self.DT` DeltaSeconds))

(fn `ChangeGameState`
  (params (State :type "/Game/KYS/EN_GameState Enum" :default "NewEnumerator3"))
  (set `self.DT` 0.0)
  (bind _output_get (set `self.GameState` State))
  (`self.StateChange` _output_get))

(fn `EventAddScore`
  (bind _output_get (set `self.PlayerScore` (+ (`self.PlayerScore`) 1)))
  (`KismetSystemLibrary.PrintString` (`KismetStringLibrary.Conv_IntToString` _output_get) true true (struct :`R` 1.0 :`G` 0.012133 :`B` 0.024673 :`A` 1.0) 5.0))

(fn `UserConstructionScript`)